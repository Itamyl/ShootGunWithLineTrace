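; Enemy actor Blueprint that tracks its health, shows it in an attached WB_EnemHealth widget, and is destroyed when health runs out.
; On BeginPlay it caches the widget from its Widget component and seeds it with current and max health.
; AnyDamage subtracts incoming damage scaled by a hundred, refreshes the widget, and destroys the actor at zero or below.
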(event `self.ReceiveBeginPlay`
  ;[1 1 1] Set health
  (bind _aswb_enem_health (cast `/Game/UI/WB_EnemHealth` (`WidgetComponent.GetUserWidgetObject` (`self.Widget`))))
  (bind _output_get (set `self.WB Health Enemy` _aswb_enem_health))
  (set `/Game/UI/WB_EnemHealth.CurrentHealth` (`self.CurrentHealth`) _output_get)
  (set `/Game/UI/WB_EnemHealth.MaxHealth` (`self.MaxHealth`) _output_get))

(event `self.ReceiveAnyDamage`
  (params (Damage :type "Float (single-precision)") (DamageType :type "DamageType Object Reference") (InstigatedBy :type "Controller Object Reference") (DamageCauser :type "Actor Object Reference"))
  (bind _output_get (set `self.CurrentHealth` (- (`self.CurrentHealth`) (* Damage 100.0))))
  (`/Game/UI/WB_EnemHealth.UpdateHealth` (`self.WB Health Enemy`) _output_get)
  (if (<= (`self.CurrentHealth`) 0)
    (`self.K2_DestroyActor`)))

(fn `UserConstructionScript`)